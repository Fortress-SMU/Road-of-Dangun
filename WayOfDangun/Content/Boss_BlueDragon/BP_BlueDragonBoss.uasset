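; Blue dragon boss actor that takes damage, shows a health bar widget, and makes a headbutt attack.
; DragonFly's heading-mode events run a looping timer that sphere-traces at FireballSpawnPoint, deals one hit, then ends the mode.
; BPCHealth handles damage and fires hurt and death responses with sounds; death hides the bar, removes DragonFly and delays actor destruction.
; Heal is a stub, and hit montage and knockback logic are disconnected.
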(event `self.Dragon Fly.OnHeadingModeTriggered`
  ;[0 0 0] 헤딩 모드 진입
  (set `self.bIsHeadingMode` true)
  (set `self.bHasAttacked` false)
  (`KismetSystemLibrary.K2_SetTimer` null "HeadingAttack" 0.1 true))

(event `self.ReceiveBeginPlay`
  ;[1 1 1] Event Begin
  (`|ExecutionSequence`
    (:`then_0`
      ;;[1 1 1] DamageEvent 등록
      (`self.Damage System Event Init`))
    (:`then_1`
      ;;[1 1 1] 드래곤 체력 바 띄우기
      (bind _returnvalue (`|CreateWidget` "/Game/UI/WBP_TempDragonHP.WBP_TempDragonHP_C"))
      (set `self.WBP_HealthBar` _returnvalue)
      (`UserWidget.AddToViewport` (`self.WBP_HealthBar`) 0))))

(event `self.Dragon Fly.OnHeadingModeEnded`
  ;[0 0 0] 헤딩 모드 종료
  (set `self.bIsHeadingMode` false)
  (`KismetSystemLibrary.K2_ClearTimer` null "HeadingAttack"))

(event `Death`
  ;[1 1 1] DamageEvent에 따른 이벤트함수
  ;;[0 0 0] 사망 처리
  (`self.HandleDeath`)
  (`Widget.SetVisibility` (`self.WBP_HealthBar`) "Hidden")
  (`ActorComponent.K2_DestroyComponent` (`self.Dragon Fly`))
  (`GameplayStatics.SpawnSoundAttached` "/Game/Boss_BlueDragon/Sounds/DragonDeathSound.DragonDeathSound" (`self.FireballSpawnPoint`) "None" (0.0 0.0 0.0) (struct) "KeepRelativeOffset" false 3.0 1.0 0.0 null null)
  (`KismetSystemLibrary.Delay` 7.0)
  (`self.K2_DestroyActor`))

(event `Blocked`
  (params (CanBeParried :type Boolean))
  ;[1 1 1] DamageEvent에 따른 이벤트함수
)

(event `Damaged`
  (params (DamageResonseInfo :type "/Game/Shared_Content/DamageSystem/S_DamageResponseInfo Structure"))
  ;[1 1 1] DamageEvent에 따른 이벤트함수
  (`GameplayStatics.SpawnSoundAttached` "/Game/Boss_BlueDragon/Sounds/DragonHurtSound__cut_4sec_.DragonHurtSound__cut_4sec_" (`self.FireballSpawnPoint`) "None" (0.0 0.0 0.0) (struct) "KeepRelativeOffset" false 1.5 1.0 0.0 null null)
  (bind _health (`self.GetCurrentHealth`))
  (set `self.Damage Causer` DamageResonseInfo_DamageCauser_6_306221674CDAC8A4A3FB94BB24E4938A)
  (set `self.isKnockedBack` DamageResonseInfo_IsKnockedBack_13_A903B075469A4EE481E996BF3E7587BC))

(fn `Damage System Event Init`
  (bind _bpc_health (`self.BPC_Health`))
  ;[1 1 1] BPC_DamageSystem에서 발신된 이벤트에, 이벤트함수 연결
  (add `/Game/Shared_Content/DamageSystem/BPC_Health.OnDeath` _bpc_health (`|CreateDelegate` :!event `Death`)) ; OnDeath이벤트에 연결
  (add `/Game/Shared_Content/DamageSystem/BPC_Health.OnBlocked` _bpc_health (`|CreateDelegate` :!event `Blocked`)) ; OnBlocked 이벤트에 연결
  (add `/Game/Shared_Content/DamageSystem/BPC_Health.OnDamaged` _bpc_health (`|CreateDelegate` :!event `Damaged`)) ; OnDamage 이벤트에 연결
)

(fn `GetCurrentHealth`
  (returns (Health :type "Float (double-precision)"))
  (return (`/Game/Shared_Content/DamageSystem/BPC_Health.Health` (`self.BPC_Health`))))

(fn `GetMaxHealth`
  (returns (MaxHealth :type "Float (double-precision)"))
  (return (`/Game/Shared_Content/DamageSystem/BPC_Health.MaxHealth` (`self.BPC_Health`))))

(fn `HeadingAttack`
  (bind _returnvalue (`SceneComponent.GetSocketLocation` (`self.FireballSpawnPoint`) "None"))
  ;[0 0 0] 조건 확인: 헤딩 모드인가? 한번 때렸는가?
  (if (`self.bIsHeadingMode`)
    (if (not (`self.bHasAttacked`))
      ;[0 0 0] 박치기 공격 & 데미지 정보 전달
      (bind (_outhit _returnvalue_2) (`KismetSystemLibrary.SphereTraceSingle` :`Start` _returnvalue :`End` _returnvalue :`Radius` 100.0 :`TraceChannel` "TraceTypeQuery4" :`TraceColor` (struct :`R` 1.0 :`G` 0.927759 :`A` 1.0) :`TraceHitColor` (struct :`R` 1.0 :`B` 0.947488 :`A` 1.0) :`DrawTime` 0.0))
      (if _returnvalue_2
        (`/Engine/EditorBlueprintResources/StandardMacros.DoOnce` false
          (:`Completed`
            (message `/Game/Shared_Content/DamageSystem/BPI_Damageable.TakeDamage` (`.HitActor` (`GameplayStatics.BreakHitResult` _outhit)) (make `/Game/Shared_Content/DamageSystem/S_DamageRequestInfo` 10.0 "NewEnumerator1" "NewEnumerator2" false true false false false self))
            (`GameplayStatics.SpawnSoundAttached` "/Game/Boss_BlueDragon/Sounds/DragonHeadingSound__cut_2sec___1_.DragonHeadingSound__cut_2sec___1_" (`self.FireballSpawnPoint`) "None" (0.0 0.0 0.0) (struct) "KeepRelativeOffset" false 1.0 0.7 0.0 null null)
            ;[0 0 0] 공격 했으니까 트레이스 끄고 헤딩 모드 종료
            (set `self.bHasAttacked` true)
            (`KismetSystemLibrary.K2_ClearTimer` null "HeadingAttack")
            (`DragonRandomFlyComponent.ForceEndHeadingMode` (`self.Dragon Fly`))))))))

(fn `Heal`
  (params (Amount :type "Float (double-precision)"))
  (returns (NewHealth :type "Float (double-precision)"))
  (return 0.0))

(fn `TakeDamage`
  (params (DamageInfo :type "/Game/Shared_Content/DamageSystem/S_DamageRequestInfo Structure"))
  (returns (WasDamaged :type Boolean))
  (bind _wasdamaged (`/Game/Shared_Content/DamageSystem/BPC_Health.TakeDamage_Execute` (`self.BPC_Health`) DamageInfo))
  (return _wasdamaged))

(fn `UserConstructionScript`)