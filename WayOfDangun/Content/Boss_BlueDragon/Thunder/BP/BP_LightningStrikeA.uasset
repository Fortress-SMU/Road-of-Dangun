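; BP_LightningStrikeA is a short-lived lightning strike hazard for the Blue Dragon boss.
; On BeginPlay it plays an attached thunder sound and a strong camera shake on player 0, then destroys itself after a brief delay.
; Its Collision overlap sends a TakeDamage message with a damage request struct, gated by DoOnce so only the first overlapping actor, unfiltered, is hit.
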(event `self.ReceiveBeginPlay`
  (`GameplayStatics.SpawnSoundAttached` "/Game/Boss_BlueDragon/Sounds/DragonLightningSound__cut_6sec_.DragonLightningSound__cut_6sec_" (`self.DefaultSceneRoot`) "None" (0.0 0.0 0.0) (struct) "KeepRelativeOffset" false 3.0 1.0 0.0 null null)
  (`LegacyCameraShake.StartLegacyCameraShake` (`GameplayStatics.GetPlayerCameraManager` 0) "/Game/Shared_Content/PlayerCharacter/CameraShake/BP_CameraShake.BP_CameraShake_C" 10.0 "World")
  (`KismetSystemLibrary.Delay` 1.5)
  (`self.K2_DestroyActor`))

(event `self.Collision.OnComponentBeginOverlap`
  (params (OverlappedComponent :type "PrimitiveComponent Object Reference") (OtherActor :type "Actor Object Reference") (OtherComp :type "PrimitiveComponent Object Reference") (OtherBodyIndex :type Integer) (bFromSweep :type Boolean) (SweepResult :type "HitResult Structure (by ref)"))
  (`/Engine/EditorBlueprintResources/StandardMacros.DoOnce` false
    (:`Completed`
      (message `/Game/Shared_Content/DamageSystem/BPI_Damageable.TakeDamage` OtherActor (make `/Game/Shared_Content/DamageSystem/S_DamageRequestInfo` 10.0 "NewEnumerator2" "NewEnumerator2" false false false false false self)))))

(fn `UserConstructionScript`)