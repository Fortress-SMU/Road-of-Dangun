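; Weather controller for the Blue Dragon boss fight that starts a lightning storm while the dragon is alive at 40% health or less.
; BeginPlay caches the first boss actor's health component, which Tick polls to run an interval timer.
; Each cycle spawns two delayed-apart lightning strikes at random spawn points.
; After the first pair, a one-time timeline fades sunlight intensity and post-process exposure compensation to change the sky.
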(event `self.ReceiveBeginPlay`
  ;[0 0 0] 번개 타이머 초기화 & 드래곤 체력 받아오기
  (set `self.LightningTimer` (`self.LightingInterval`))
  (bind _outactors (`GameplayStatics.GetAllActorsOfClass` "/Game/Boss_BlueDragon/BP_BlueDragonBoss.BP_BlueDragonBoss_C"))
  (bind _asbp_blue_dragon_boss (cast `/Game/Boss_BlueDragon/BP_BlueDragonBoss` (`|GetArrayItem` _outactors)))
  (set `self.BP BlueDragon` null)
  (set `self.BPC Health` (`/Game/Boss_BlueDragon/BP_BlueDragonBoss.BPC_Health` _asbp_blue_dragon_boss)))

(event `self.ReceiveTick`
  (params (DeltaSeconds :type "Float (single-precision)"))
  (bind _lightningspawnpoints (`self.LightningSpawnPoints`))
  (bind _bpc_health (`self.BPC Health`))
  (bind _returnvalue (/ (`/Game/Shared_Content/DamageSystem/BPC_Health.Health` _bpc_health) (`/Game/Shared_Content/DamageSystem/BPC_Health.MaxHealth` _bpc_health)))
  (bind _returnvalue_2 (- (`KismetArrayLibrary.Array_Length` _lightningspawnpoints) 1))
  ;[0.2719 0.2646 0] 일정 간격으로 두 번씩 번개 치기
  (if (`KismetMathLibrary.Conv_IntToBool` (`KismetMathLibrary.And_IntInt` (`KismetMathLibrary.Conv_BoolToInt` (> _returnvalue 0.0)) (`KismetMathLibrary.Conv_BoolToInt` (<= _returnvalue 0.4))))
    (bind _output_get (set `self.LightningTimer` (- (`self.LightningTimer`) DeltaSeconds)))
    (if (<= _output_get 0.0)
      (`|SpawnActorFromClass` "/Game/Boss_BlueDragon/Thunder/BP/BP_LightningStrikeA.BP_LightningStrikeA_C" (`KismetMathLibrary.Conv_VectorToTransform` (`self.K2_GetActorLocation` (`|GetArrayItem` _lightningspawnpoints (`KismetMathLibrary.RandomIntegerInRange` 0 _returnvalue_2)))) "Undefined" "MultiplyWithRoot" null null)
      (set `self.LightningTimer` (`self.LightingInterval`))
      (`KismetSystemLibrary.Delay` 1.0)
      (`|SpawnActorFromClass` "/Game/Boss_BlueDragon/Thunder/BP/BP_LightningStrikeA.BP_LightningStrikeA_C" (`KismetMathLibrary.Conv_VectorToTransform` (`self.K2_GetActorLocation` (`|GetArrayItem` _lightningspawnpoints (`KismetMathLibrary.RandomIntegerInRange` 0 _returnvalue_2)))) "Undefined" "MultiplyWithRoot" null null)
      ;[0.2948 0.4469 1] 하늘 서서히 어둡게 변경
      (`/Engine/EditorBlueprintResources/StandardMacros.DoOnce` false
        (:`Completed`
          (bind (_direction _sky_light _exposure) (`Timeline|Light Fade`)
            (:`Update`
              (`LightComponent.SetIntensity` (`Light.LightComponent` (`self.SunLight`)) _sky_light)
              (bind _output_get_2 (set `PostProcessVolume.Settings` (struct) (`self.PostProcessVolume`)))
              (bind _structout (setmembers `PostProcessSettings` :`StructRef` _output_get_2 :`AutoExposureBias` _exposure))
              (set `PostProcessVolume.Settings` _structout (`self.PostProcessVolume`)))))))))

(fn `UserConstructionScript`)