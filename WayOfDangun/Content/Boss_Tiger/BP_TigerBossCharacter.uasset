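; Tiger boss (Jangsanbeom) character that creates its health bar widget and broadcasts HP every tick.
; Damage requests go to BPCHealth, whose events drive death handling and flag-gated timeline knockback along the attacker's forward vector.
; A looping timer at the frame interval repeats claw box traces between start and stop calls.
; CPP-suffixed events trigger jump-dash sphere traces or stop tracing; an already-hit list prevents duplicate damage.
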(event `self.ReceiveBeginPlay`
  ;[1 1 1] Event Begin
  (`|ExecutionSequence`
    (:`then_0`
      ;;[1 1 1] DamageEvent 등록
      (`self.Damage System Event Init`))
    (:`then_1`
      ;;[1 1 1] 장산범 체력 바 띄우기
      (bind _returnvalue (`|CreateWidget` "/Game/UI/WBP_TGBossHealthBar.WBP_TGBossHealthBar_C"))
      (set `self.WBP_HealthBar` _returnvalue)
      (`UserWidget.AddToViewport` (`self.WBP_HealthBar`) 0))))

(event `CustomEvent`
  ;[1 1 1] AttackEvent 등록 (BP로 동작함)
  (`self.Attack_Claw`))

(event `self.ReceiveTick`
  (params (DeltaSeconds :type "Float (single-precision)"))
  ;[1 1 1] Event Tick
  (set `self.curDeltaTime` DeltaSeconds)
  (`self.callDelegate` (`/Game/Shared_Content/DamageSystem/BPC_Health.Health` (`self.BPC_Health`)) (`/Game/Shared_Content/DamageSystem/BPC_Health.MaxHealth` (`self.BPC_Health`))))

(event `Death`
  ;[1 1 1] DamageEvent에 따른 이벤트함수
  (`self.Dead`)
  (`Widget.SetVisibility` (`self.WBP_HealthBar`) "Hidden"))

(event `Blocked`
  (params (CanBeParried :type Boolean))
  ;[1 1 1] DamageEvent에 따른 이벤트함수
)

(event `Damaged`
  (params (DamageResonseInfo :type "/Game/Shared_Content/DamageSystem/S_DamageResponseInfo Structure"))
  (bind (_velocity_x _velocity_y _velocity_z) (`KismetMathLibrary.BreakVector` (`MovementComponent.Velocity` (`self.CharacterMovement`))))
  ;[1 1 1] DamageEvent에 따른 이벤트함수
  (bind _health (`self.GetCurrentHealth`))
  (set `self.Damage Causer` DamageResonseInfo_DamageCauser_6_306221674CDAC8A4A3FB94BB24E4938A)
  ;[1 1 1] 넉백
  (if (`self.isKnockedBack`)
    (bind _output_get (set `self.curDamagedLocation` (`self.GetActorForwardVector` (`self.Damage Causer`)))) ; DamageCauser가 시간지나면 사라지는 액터일 경우를 대비해서\n미리 값을 받아둠
    (bind (_direction _distancemutiplier) (`Timeline|타임라인_1` :!via `PlayFromStart`)
      (:`Update`
        (bind (_returnvalue_x _returnvalue_y) (`KismetMathLibrary.BreakVector` (* _output_get (* _distancemutiplier 40000.0))))
        (set `MovementComponent.Velocity` (`KismetMathLibrary.MakeVector` _returnvalue_x _returnvalue_y _velocity_z) (`self.CharacterMovement`))))))

(event `StartAttackTrace`
  ;[1 1 1] Comment
  (bind _returnvalue (`KismetSystemLibrary.K2_SetTimerDelegate` (delegate `CreateAttackTrace`) (`self.curDeltaTime`) true))
  (set `self.AttackTimerHandler` _returnvalue))

(event `self.CreateAttackTraceCPP`
  ;[1 1 1] Comment
  (`self.Attack_JumpDash`))

(event `CreateAttackTrace`
  ;[1 1 1] Comment
  (`self.Attack_Claw`))

(event `self.StopAttackTraceCPP`
  ;[1 1 1] Comment
  (`KismetSystemLibrary.K2_ClearAndInvalidateTimerHandle` (`self.AttackTimerHandler`))
  (`KismetArrayLibrary.Array_Clear` (`self.AlreadyHitActor`)))

(event `StopAttackTrace`
  ;[1 1 1] Comment
  (`KismetSystemLibrary.K2_ClearAndInvalidateTimerHandle` (`self.AttackTimerHandler`))
  (`KismetArrayLibrary.Array_Clear` (`self.AlreadyHitActor`)))

(fn `Attack_Claw`
  (bind _alreadyhitactor (`self.AlreadyHitActor`))
  (bind _attackrange_claw (`self.AttackRange_Claw`))
  (bind _returnvalue (`SceneComponent.K2_GetComponentLocation` (`self.AttackRange_Claw`)))
  ;[1 1 1] Claw 공격트레이스 생성
  (bind (_outhit _returnvalue_2) (`KismetSystemLibrary.BoxTraceSingle` :`Start` _returnvalue :`End` (+ _returnvalue (* (`KismetMathLibrary.Vector_Forward`) 1.0)) :`HalfSize` (`BoxComponent.GetScaledBoxExtent` _attackrange_claw) :`Orientation` (`SceneComponent.K2_GetComponentRotation` _attackrange_claw) :`TraceChannel` "TraceTypeQuery4" :`TraceColor` (struct :`R` 1.0 :`B` 0.964686) :`TraceHitColor` (struct :`G` 0.296138 :`B` 1.0) :`DrawTime` 0.0)) ; AttackTraceRange의 위치/크기를 가져와서,\n해당 위치에 박스트레이스를 생성
  (if _returnvalue_2
    (bind (_bblockinghit _binitialoverlap _time _distance _location _impactpoint _normal _impactnormal _physmat _hitactor) (`GameplayStatics.BreakHitResult` _outhit))
    (bind _output_get (set `self.curHitActor` _hitactor)) ; 피격된 대상 저장
    ;;[1 1 1] AttackTrace에 공격 중복적용 방지
    (if (not (`KismetArrayLibrary.Array_Contains` _alreadyhitactor _hitactor))
      (`KismetArrayLibrary.Array_Add` _alreadyhitactor _output_get)
      (message `/Game/Shared_Content/DamageSystem/BPI_Damageable.TakeDamage` (`self.curHitActor`) (make `/Game/Shared_Content/DamageSystem/S_DamageRequestInfo` 10.0 "NewEnumerator1" "NewEnumerator2" false true false false false self)) ; 데미지 적용
    )))

(fn `Attack_JumpDash`
  (bind _returnvalue (`self.K2_GetActorLocation`))
  (bind _alreadyhitactor (`self.AlreadyHitActor`))
  ;[1 1 1] Claw 공격트레이스 생성
  (bind (_outhit _returnvalue_2) (`KismetSystemLibrary.SphereTraceSingle` :`Start` _returnvalue :`End` (+ _returnvalue (* (`self.GetActorForwardVector`) 300.0)) :`Radius` 420.0 :`TraceChannel` "TraceTypeQuery4" :`TraceColor` (struct :`R` 1.0) :`TraceHitColor` (struct :`G` 1.0) :`DrawTime` 0.0))
  (if _returnvalue_2
    (bind (_bblockinghit _binitialoverlap _time _distance _location _impactpoint _normal _impactnormal _physmat _hitactor) (`GameplayStatics.BreakHitResult` _outhit))
    (bind _output_get (set `self.curHitActor` _hitactor)) ; 피격된 대상 저장
    ;;[1 1 1] AttackTrace에 공격 중복적용 방지
    (if (not (`KismetArrayLibrary.Array_Contains` _alreadyhitactor _hitactor))
      (`KismetArrayLibrary.Array_Add` _alreadyhitactor _output_get)
      (message `/Game/Shared_Content/DamageSystem/BPI_Damageable.TakeDamage` (`self.curHitActor`) (make `/Game/Shared_Content/DamageSystem/S_DamageRequestInfo` 10.0 "NewEnumerator1" "NewEnumerator2" false true false false false self)) ; 데미지 적용
    )))

(fn `Damage System Event Init`
  (bind _bpc_health (`self.BPC_Health`))
  ;[1 1 1] BPC_DamageSystem에서 발신된 이벤트에, 이벤트함수 연결
  (add `/Game/Shared_Content/DamageSystem/BPC_Health.OnDeath` _bpc_health (`|CreateDelegate` :!event `Death`)) ; OnDeath이벤트에 연결
  (add `/Game/Shared_Content/DamageSystem/BPC_Health.OnBlocked` _bpc_health (`|CreateDelegate` :!event `Blocked`)) ; OnBlocked 이벤트에 연결
  (add `/Game/Shared_Content/DamageSystem/BPC_Health.OnDamaged` _bpc_health (`|CreateDelegate` :!event `Damaged`)) ; OnDamage 이벤트에 연결
)

(fn `GetCurrentHealth`
  (returns (Health :type "Float (double-precision)"))
  (return (`/Game/Shared_Content/DamageSystem/BPC_Health.Health` (`self.BPC_Health`))))

(fn `GetMaxHealth`
  (returns (MaxHealth :type "Float (double-precision)"))
  (return (`/Game/Shared_Content/DamageSystem/BPC_Health.MaxHealth` (`self.BPC_Health`))))

(fn `Heal`
  (params (Amount :type "Float (double-precision)"))
  (returns (NewHealth :type "Float (double-precision)"))
  (return 0.0))

(fn `TakeDamage`
  (params (DamageInfo :type "/Game/Shared_Content/DamageSystem/S_DamageRequestInfo Structure"))
  (returns (WasDamaged :type Boolean))
  (`/Game/Shared_Content/DamageSystem/BPC_Health.TakeDamage_Execute` (`self.BPC_Health`) DamageInfo)
  (return false))

(fn `UserConstructionScript`)