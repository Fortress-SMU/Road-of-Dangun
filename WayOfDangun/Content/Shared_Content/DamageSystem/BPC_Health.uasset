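; BPC_Health is a health component that tracks an owner's health and death state, handling healing and incoming damage.
; TakeDamageExecute runs each damage info struct through CheckDamageConditions, which weighs death, invincibility and blocking to block, apply or ignore the hit.
; Results go out through event dispatchers: OnBlocked with parry eligibility, OnDeath at zero health, and OnDamaged with hit-response info only when interruptible or force-interrupted.
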(fn `Heal_Execute`
  (params (Amount :type "Float (double-precision)"))
  (returns (NewHealth :type "Float (double-precision)"))
  (if (not (`self.IsDead`))
    (bind _output_get (set `self.Health` (`KismetMathLibrary.FClamp` (+ Amount (`self.Health`)) 0.0 (`self.MaxHealth`))))
    (return _output_get)))

(fn `TakeDamage_Execute`
  (params (DamageInfo :type "/Game/Shared_Content/DamageSystem/S_DamageRequestInfo Structure"))
  (returns (WasDamaged :type Boolean))
  (bind (_amount _damagetype _hitreaction _shoulddamagedinvincible _isknockedback _canbeblocked _canbeparried _shouldforecinterrupt _damagecauser) (break `/Game/Shared_Content/DamageSystem/S_DamageRequestInfo` DamageInfo))
  (`self.CheckDamageConditions` _shoulddamagedinvincible _canbeblocked ; 데미지 적용 가능한지 판정
    (:`BlockDamage`
      ;[1 1 1] 1. 데미지 막힘 - 이벤트 발신 (OnBlocked)
      (`self.OnBlocked` _canbeparried) ; 1. Blocked 이벤트 발신
      (return false))
    (:`DoDamage`
      ;[1 1 1] 2. 데미지 적용O - 이벤트 발신 (OnDamageResponse/OnDeath)
      (bind _output_get (set `self.Health` (- (`self.Health`) _amount)))
      (if (<= _output_get 0.0)
        (set `self.IsDead` true)
        (`self.OnDeath`) ; 2. Death 이벤트 발신
        (return true)
        (elif (or (`self.IsInterruptible`) _shouldforecinterrupt)
          (`self.OnDamaged` (make `/Game/Shared_Content/DamageSystem/S_DamageResponseInfo` _damagecauser _hitreaction (0.0 0.0 0.0) _isknockedback)) ; 3. DamageResponse 이벤트 발신
          (return true))))
    (:`NoDamage`
      ;[1 1 1] 3. 데미지 적용X ("무적" 혹은 "방어 성공")
      (return false))))