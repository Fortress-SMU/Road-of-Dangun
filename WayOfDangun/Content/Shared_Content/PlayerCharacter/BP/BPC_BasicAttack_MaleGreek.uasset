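; Player component for the MaleGreek character's four-step hammer combo attack, triggered by input when the hammer is in hand and stamina suffices.
; Each montage's CanNextAttack notify re-enables input and advances the combo counter, while a timer resets the combo.
; Montage-driven start/stop events run a looping sphere trace at the hammer head.
; Hits deal damage once per actor per swing, with knockback, sound and camera shake.
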(event `self.ReceiveBeginPlay`
  ;[1 1 1] Event Begin
  (`|ExecutionSequence`
    (:`then_0`
      ;;[1 1 1] Owner 오브젝트 참조
      (bind _asbp_male_greek (cast `/Game/Shared_Content/PlayerCharacter/BP/BP_MaleGreek` (`self.GetOwner`)))
      (bind _output_get (set `self.BP_PlayerCharacter` _asbp_male_greek))
      (set `self.CharacterMesh` (`Character.Mesh` _output_get)))
    (:`then_1`
      ;;[1 1 1] BP_MaleGreek의 액터 컴포넌트 참조
      (set `self.FollowCameraComponent` (`/Game/Shared_Content/PlayerCharacter/BP/BP_MaleGreek.FollowCamera` (`self.BP_PlayerCharacter`))))
    (:`then_2`
      ;;[1 1 1] ABP_PlayerCharacter 초기화
      (bind _asabp_hammer_male_greek (cast `/Game/Shared_Content/PlayerCharacter/BP/ABP_HammerMaleGreek` (`SkeletalMeshComponent.GetAnimInstance` (`Character.Mesh` (`self.BP_PlayerCharacter`)))))
      (set `self.ABP_PlayerCharacter` _asabp_hammer_male_greek))))

(event `self.ReceiveTick`
  (params (DeltaSeconds :type "Float (single-precision)"))
  ;[1 1 1] Event Tick
  (set `self.curDeltaTime` DeltaSeconds))

(event `EnhancedInput|/Game/Shared_Content/Input/IA_MyAttack`
  (params (ActionValue :type Boolean) (ElapsedSeconds :type "Float (double-precision)") (TriggeredSeconds :type "Float (double-precision)") (InputAction :type "InputAction Object Reference" :default "/Game/Shared_Content/Input/IA_MyAttack.IA_MyAttack"))
  ;[1 1 1] 기본공격 - 콤보 애니메이션
  (:`Triggered`
    (if (`/Game/Shared_Content/PlayerCharacter/BP/BP_MaleGreek.isHammerOnHand` (`self.BP_PlayerCharacter`))
      (if (`self.canAttack`)
        ;;[1 1 1] 스테미나 검사
        (bind _returnisstaminaenough (`/Game/Shared_Content/PlayerCharacter/BP/BP_MaleGreek.Use Stamina` (`self.BP_PlayerCharacter`) 20.0))
        (if _returnisstaminaenough
          (set `self.canAttack` false)
          (`KismetArrayLibrary.Array_Clear` (`self.AlreadyHitActors`)) ; AlreaddyHitActors 배열을 비움
          (set `/Game/Shared_Content/PlayerCharacter/BP/BP_MaleGreek.canUpdateCharacterForward` true (`self.BP_PlayerCharacter`))
          (switch `int` (`self.ComboCounter`)
            (:`0`
              (bind _notifyname (`|PlayMontage` (`self.CharacterMesh`) "/Game/Shared_Content/PlayerCharacter/Animation/HammerAnimation/Montages/001Hammer_Combo03_1_Retargeted_Montage.001Hammer_Combo03_1_Retargeted_Montage" 1.0 1.5)
                (:`then`
                  (`KismetSystemLibrary.K2_SetTimerDelegate` (delegate `ResetCounter`) 2.5 :!label _label))
                (:`OnNotifyBegin`
                  (`self.CurComboFinsih` _notifyname 1))))
            (:`1`
              (bind _notifyname_2 (`|PlayMontage` (`self.CharacterMesh`) "/Game/Shared_Content/PlayerCharacter/Animation/HammerAnimation/Montages/001Hammer_Combo03_2_Retargeted_Montage.001Hammer_Combo03_2_Retargeted_Montage")
                (:`then`
                  (goto _label))
                (:`OnNotifyBegin`
                  (`self.CurComboFinsih` _notifyname_2 2))))
            (:`2`
              (bind _notifyname_3 (`|PlayMontage` (`self.CharacterMesh`) "/Game/Shared_Content/PlayerCharacter/Animation/HammerAnimation/Montages/001Hammer_Combo03_3_Retargeted_Montage.001Hammer_Combo03_3_Retargeted_Montage")
                (:`then`
                  (goto _label))
                (:`OnNotifyBegin`
                  (`self.CurComboFinsih` _notifyname_3 3))))
            (:`3`
              (bind _notifyname_4 (`|PlayMontage` (`self.CharacterMesh`) "/Game/Shared_Content/PlayerCharacter/Animation/HammerAnimation/Montages/001Hammer_Combo03_4_Retargeted_Montage.001Hammer_Combo03_4_Retargeted_Montage" 1.0 0.95)
                (:`then`
                  (goto _label))
                (:`OnNotifyBegin`
                  (`self.CurComboFinsih` _notifyname_4))))))))))

(event `ResetCounter`
  ;[1 1 1] 기본공격 - 콤보 애니메이션
  (set `self.ComboCounter` 0)
  (set `self.canAttack` true)
  (set `/Game/Shared_Content/PlayerCharacter/BP/BP_MaleGreek.canUpdateCharacterForward` false (`self.BP_PlayerCharacter`)))

(event `AttackReset`
  ;[1 1 1] 기본공격 - 콤보 애니메이션
  (if true
    (set `self.canAttack` true) ; 공격 몽타주가
    (set `self.ComboCounter` 0)))

(event `StartAttackTrace`
  ;[1 1 1] 기본공격 - 공격 트레이스 생성 (애니메이션 몽타주로 실행)
  (bind _returnvalue (`KismetSystemLibrary.K2_SetTimerDelegate` (delegate `AttackTrace`) (`self.curDeltaTime`) true))
  (set `self.AttackTimerHandler` _returnvalue))

(event `AttackTrace`
  (bind _alreadyhitactors (`self.AlreadyHitActors`))
  (bind _hammerattackrange (`/Game/Shared_Content/PlayerCharacter/BP/BP_MaleGreek.HammerAttackRange` (`self.BP_PlayerCharacter`)))
  ;[1 1 1] 기본공격 - 공격 트레이스 생성 (애니메이션 몽타주로 실행)
  (bind (_outhit _returnvalue) (`KismetSystemLibrary.SphereTraceSingle` :`Start` (`SceneComponent.K2_GetComponentLocation` _hammerattackrange) :`End` (`KismetMathLibrary.TransformLocation` (`SceneComponent.K2_GetComponentToWorld` _hammerattackrange) (+ (`SceneComponent.RelativeLocation` _hammerattackrange) (75.0 0.0 0.0))) :`Radius` 65.0 :`TraceChannel` "TraceTypeQuery3" :`DrawTime` 0.0)) ; 트레이스 생성
  (if _returnvalue
    (bind (_bblockinghit _binitialoverlap _time _distance _location _impactpoint _normal _impactnormal _physmat _hitactor) (`GameplayStatics.BreakHitResult` _outhit))
    (set `self.curHitActor` _hitactor) ; 피격된 대상 저장
    ;;[1 1 1] AttackTrace에 공격 중복적용 방지
    (if (not (`KismetArrayLibrary.Array_Contains` _alreadyhitactors _hitactor))
      (`KismetArrayLibrary.Array_Add` _alreadyhitactors _hitactor)
      ;;[1 1 1] 데미지 적용
      (message `/Game/Shared_Content/DamageSystem/BPI_Damageable.TakeDamage` (`self.curHitActor`) (make `/Game/Shared_Content/DamageSystem/S_DamageRequestInfo` 10.0 "NewEnumerator1" "NewEnumerator2" false true false false false (`self.BP_PlayerCharacter`)))
      ;;[1 1 1] VFX/SFX
      (`GameplayStatics.PlaySoundAtLocation` "/Game/Shared_Content/PlayerCharacter/SFX/Explosion01.Explosion01" _location (struct) 2.0 20.0 0.0 null null null null)
      (`LegacyCameraShake.StartLegacyCameraShake` (`GameplayStatics.GetPlayerCameraManager` 0) "/Game/Shared_Content/PlayerCharacter/CameraShake/BP_CameraShake.BP_CameraShake_C" 3.0 "World"))))

(event `StopAttackTrace`
  ;[1 1 1] 기본공격 - 공격 트레이스 제거 (애니메이션 몽타주로 실행)
  (`KismetSystemLibrary.K2_ClearAndInvalidateTimerHandle` (`self.AttackTimerHandler`)))

(fn `CurComboFinsih`
  (params (ArgNotifyName :type Name) (NextComboCounter :type Integer))
  (if (== ArgNotifyName "CanNextAttack")
    (set `self.canAttack` true)
    (set `self.ComboCounter` NextComboCounter)))