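; Player component for BP_MaleGreek that handles throwing and recalling the hammer with the right mouse button.
; If stamina allows, a throw plays a montage, briefly enables character forward updating, then spawns BP_ThrownHammer at the launch point along follow-camera rotation and hides the held hammer.
; When the hand is empty, the button tells the thrown hammer to return.
; ReciveHammer marks it in hand and plays the catch montage.
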(event `self.ReceiveBeginPlay`
  (bind _bp_playercharacter (`self.BP_PlayerCharacter`))
  ;[1 1 1] Event Begin
  ;;[1 1 1] BP_MaleGreek와 액터컴포넌트 참조
  (bind _asbp_male_greek (cast `/Game/Shared_Content/PlayerCharacter/BP/BP_MaleGreek` (`self.GetOwner`)))
  (set `self.BP_PlayerCharacter` _asbp_male_greek)
  (`|ExecutionSequence`
    (:`then_0`
      (set `self.FollowCameraComponent` (`/Game/Shared_Content/PlayerCharacter/BP/BP_MaleGreek.FollowCamera` _bp_playercharacter)))
    (:`then_1`
      (set `self.HammerLaunchPoint` (`/Game/Shared_Content/PlayerCharacter/BP/BP_MaleGreek.HammerLaunchPoint` _bp_playercharacter)))
    (:`then_2`
      (set `self.handedHammer` (`/Game/Shared_Content/PlayerCharacter/BP/BP_MaleGreek.Hammer` _bp_playercharacter)))))

(event `Key|RightMouseButton`
  (params (Key :type "Key Structure"))
  (bind _returnvalue_location (`KismetMathLibrary.BreakTransform` (`SceneComponent.K2_GetComponentToWorld` (`self.HammerLaunchPoint`))))
  (bind (_returnvalue_location_2 _returnvalue_rotation) (`KismetMathLibrary.BreakTransform` (`SceneComponent.K2_GetComponentToWorld` (`self.FollowCameraComponent`))))
  ;[1 1 1] Throw/Recall Hammer (망치 던지기/리콜)
  (:`Pressed`
    (if (`/Game/Shared_Content/PlayerCharacter/BP/BP_MaleGreek.isHammerOnHand` (`self.BP_PlayerCharacter`))
      ;;[1 1 1] 망치 던지기
      (bind _returnisstaminaenough (`/Game/Shared_Content/PlayerCharacter/BP/BP_MaleGreek.Use Stamina` (`self.BP_PlayerCharacter`) 70.0)) ; 소비 스테미나 70으로 할 것
      (if _returnisstaminaenough
        (set `/Game/Shared_Content/PlayerCharacter/BP/BP_MaleGreek.isHammerOnHand` false (`self.BP_PlayerCharacter`))
        (set `/Game/Shared_Content/PlayerCharacter/BP/BP_MaleGreek.canUpdateCharacterForward` true (`self.BP_PlayerCharacter`))
        (`Character.PlayAnimMontage` (`self.BP_PlayerCharacter`) "/Game/Shared_Content/PlayerCharacter/Animation/HammerAnimation/Montages/001Hammer_ThrowHammer_Montage.001Hammer_ThrowHammer_Montage" 1.0 "None")
        (`KismetSystemLibrary.Delay` 0.64)
        (set `/Game/Shared_Content/PlayerCharacter/BP/BP_MaleGreek.canUpdateCharacterForward` false (`self.BP_PlayerCharacter`))
        (bind _returnvalue (`|SpawnActorFromClass` "/Game/Shared_Content/PlayerCharacter/BP/BP_ThrownHammer.BP_ThrownHammer_C" (`KismetMathLibrary.MakeTransform` (+ _returnvalue_location (0.0 0.0 0.0)) _returnvalue_rotation) "AlwaysSpawn" "MultiplyWithRoot" null null))
        (set `self.curThrowedHammer` _returnvalue)
        (`SceneComponent.SetVisibility` (`self.handedHammer`) false false) ; 플레이어가 들고 있는 망치 안 보이도록
      )
      (else
        ;;[1 1 1] 망치 리콜
        (bind _curthrowedhammer (`self.curThrowedHammer`)
          (:`then`
            (`/Game/Shared_Content/PlayerCharacter/BP/BP_ThrownHammer.ReturnHammerToPlayer` _curthrowedhammer))
          (:`else`))))))

(event `ReciveHammer`
  ;[1 1 1] Throw/Recall Hammer (망치 던지기/리콜)
  ;;[1 1 1] 망치 리콜
  ;;;[1 1 1] 돌아오는 시간이 지나면 회수 애니메이션 실행
  (set `/Game/Shared_Content/PlayerCharacter/BP/BP_MaleGreek.isHammerOnHand` true (`self.BP_PlayerCharacter`))
  (`Character.PlayAnimMontage` (`self.BP_PlayerCharacter`) "/Game/Shared_Content/PlayerCharacter/Animation/HammerAnimation/Montages/001Hammer_Receive_Montage.001Hammer_Receive_Montage" 0.7 "None"))