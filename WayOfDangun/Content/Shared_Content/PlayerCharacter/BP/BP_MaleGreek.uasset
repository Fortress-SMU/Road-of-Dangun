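; Player character Blueprint for the hammer-wielding male Greek, handling Enhanced Input movement, camera look, jumping and a stamina-costed roll.
; BPCHealth handles damage and healing, sending events back for hit reactions that reset BPCBasicAttackMaleGreek attacks, and for death with its UI.
; Timelines drive roll and knockback velocity.
; Tick regenerates stamina outside attack and dodge montage slots via a Delay throttle, and optionally turns the body toward camera yaw.
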(event `self.ReceiveTick`
  (params (DeltaSeconds :type "Float (single-precision)"))
  ;[1 1 1] Event Tick
  (`self.IncreaseStamina`)
  (if (`self.canUpdateCharacterForward`)
    (`self.UpdateCharacterForwrdByCamera`)))

(event `self.ReceiveBeginPlay`
  ;[1 1 1] Event Begin
  (`|ExecutionSequence`
    (:`then_0`
      ;;[1 1 1] InputMappingContext 연결
      (bind _asplayer_controller (cast `PlayerController` (`self.GetController`)))
      (message `EnhancedInputSubsystemInterface.AddMappingContext` (pcsubsystem `EnhancedInputLocalPlayerSubsystem` _asplayer_controller) "/Game/Shared_Content/Input/IMC_MaleGreek.IMC_MaleGreek" 0 (struct)))
    (:`then_1`
      ;;[1 1 1] Damage System "이벤트-이벤트함수" 연결
      (`self.Damage System Event Init`))
    (:`then_2`
      ;;[1 1 1] 상태바를 뷰포트에 표시
      (bind _returnvalue (`|CreateWidget` "/Game/UI/WBP_StatusBar.WBP_StatusBar_C"))
      (`UserWidget.AddToViewport` _returnvalue 0))
    (:`then_3`
      ;;[1 1 1] ABP_PlayerCharacter 초기화
      (bind _asabp_hammer_male_greek (cast `/Game/Shared_Content/PlayerCharacter/BP/ABP_HammerMaleGreek` (`SkeletalMeshComponent.GetAnimInstance` (`self.Mesh`))))
      (set `self.ABP_PlayerCharacter` _asabp_hammer_male_greek))))

(event `Key|W`
  (params (Key :type "Key Structure"))
  ;[1 1 1] Event Tick
)

(event `Death`
  ;[1 1 1] DamageEvent 수신
  (`|PlayMontage` (`self.Mesh`) "/Game/Shared_Content/PlayerCharacter/Animation/HammerAnimation/Montages/Deaddead02_Retargeted_Montage.Deaddead02_Retargeted_Montage"
    (:`then`
      (`self.DisableInput` null)
      ;;[1 1 1] 나중에 GameMode 블루프린트로 옮기기
      (`KismetSystemLibrary.Delay` 3.0)
      (set `PlayerController.bShowMouseCursor` true (`GameplayStatics.GetPlayerController` 0))
      (bind _returnvalue (`|CreateWidget` "/Game/UI/Dead.Dead_C"))
      (`UserWidget.AddToViewport` _returnvalue 0))))

(event `Blocked`
  (params (CanBeParried :type Boolean))
  ;[1 1 1] DamageEvent 수신
)

(event `Damaged`
  (params (DamageResponseInfo :type "/Game/Shared_Content/DamageSystem/S_DamageResponseInfo Structure"))
  (bind (_velocity_x _velocity_y _velocity_z) (`KismetMathLibrary.BreakVector` (`MovementComponent.Velocity` (`self.CharacterMovement`))))
  ;[1 1 1] DamageEvent 수신
  (`/Game/Shared_Content/PlayerCharacter/BP/BPC_BasicAttack_MaleGreek.AttackReset` (`self.BPC_BasicAttack_MaleGreek`)) ; 공격 중이었다면\n공격세팅 초기화
  (set `self.DamageCauser` DamageResponseInfo_DamageCauser_6_306221674CDAC8A4A3FB94BB24E4938A)
  (set `self.isKnockedBack` DamageResponseInfo_IsKnockedBack_13_A903B075469A4EE481E996BF3E7587BC)
  (bind _health (`self.GetCurrentHealth`))
  ;;[1 1 1] 피격 애니메이션
  (`|PlayMontage` (`self.Mesh`) "/Game/Shared_Content/PlayerCharacter/Animation/HammerAnimation/Montages/Damagedhit_body_back_Retargeted_Montage.Damagedhit_body_back_Retargeted_Montage"
    (:`then`
      ;;[1 1 1] 넉백 적용
      (if (`self.isKnockedBack`)
        (bind _output_get (set `self.curDamagedLocation` (`self.GetActorForwardVector` (`self.DamageCauser`))))
        (bind (_direction _distancemultiplier) (`Timeline|Timeline_0` :!via `PlayFromStart`)
          (:`Update`
            (bind (_returnvalue_x _returnvalue_y) (`KismetMathLibrary.BreakVector` (* _output_get (* _distancemultiplier 4000.0))))
            (set `MovementComponent.Velocity` (`KismetMathLibrary.MakeVector` _returnvalue_x _returnvalue_y _velocity_z) (`self.CharacterMovement`))))))))

(event `IncreaseStamina`
  ;[1 1 1] Stamina System (스테미나 시스템)
  ;;[1 1 1] Stamina Recovery (Idle/Move 애니메이션에서만 실행)
  (`KismetSystemLibrary.Delay` 0.05)
  (set `self.canRecoveryStamina` (and (not (`AnimInstance.IsSlotActive` (`self.ABP_PlayerCharacter`) "DefaultSlot")) (not (`AnimInstance.IsSlotActive` (`self.ABP_PlayerCharacter`) "BasicComboAttack")))) ; 애니메이션 몽타주가 공격/회피 슬롯이면, 스테미나 회복 불가
  (if (`self.canRecoveryStamina`)
    (set `self.curStamina` (`KismetMathLibrary.FClamp` (+ (`self.curStamina`) (`self.staminaRecoveryAmount`)) 0.0 (`self.maxStamina`)))))

(event `EnhancedInput|/Game/Shared_Content/Input/IA_MyLookAround`
  (params (ActionValue :type "Vector2D Structure") (ElapsedSeconds :type "Float (double-precision)") (TriggeredSeconds :type "Float (double-precision)") (InputAction :type "InputAction Object Reference" :default "/Game/Shared_Content/Input/IA_MyLookAround.IA_MyLookAround"))
  ;[1 1 1] Basic Move (기본 동작)
  ;;[1 1 1] Input_LookAround
  (:`Triggered`
    (`self.AddControllerYawInput` (* ActionValue_X (`self.lookAroundSpeedX`)))
    (`self.AddControllerPitchInput` (* (* ActionValue_Y (`self.lookAroundSpeedY`)) -1.0))))

(event `EnhancedInput|/Game/Shared_Content/Input/IA_MyMovement`
  (params (ActionValue :type "Vector2D Structure") (ElapsedSeconds :type "Float (double-precision)") (TriggeredSeconds :type "Float (double-precision)") (InputAction :type "InputAction Object Reference" :default "/Game/Shared_Content/Input/IA_MyMovement.IA_MyMovement"))
  (bind (_returnvalue_roll _returnvalue_pitch _returnvalue_yaw) (`KismetMathLibrary.BreakRotator` (`self.GetControlRotation`)))
  (bind (_returnvalue_roll_2 _returnvalue_pitch_2 _returnvalue_yaw_2) (`KismetMathLibrary.BreakRotator` (`self.GetControlRotation`)))
  ;[1 1 1] Basic Move (기본 동작)
  ;;[1 1 1] Input_Movement
  (:`Triggered`
    (`self.AddMovementInput` (`KismetMathLibrary.GetRightVector` (`KismetMathLibrary.MakeRotator` _returnvalue_roll_2 0.0 _returnvalue_yaw_2)) ActionValue_X)
    (`self.AddMovementInput` (`KismetMathLibrary.GetForwardVector` (`KismetMathLibrary.MakeRotator` 0.0 0.0 _returnvalue_yaw)) ActionValue_Y)))

(event `Key|LeftShift`
  (params (Key :type "Key Structure"))
  (bind (_velocity_x _velocity_y _velocity_z) (`KismetMathLibrary.BreakVector` (`MovementComponent.Velocity` (`self.CharacterMovement`))))
  ;[1 1 1] Dodge (구르기)
  (:`Pressed`
    ;;[1 1 1] 구르기 중에, 구르기 재실행 방지
    (if (`self.canDodge`)
      (bind _returnisstaminaenough (`self.Use Stamina` 30.0))
      (if _returnisstaminaenough
        (set `self.canDodge` false)
        (`/Game/Shared_Content/PlayerCharacter/BP/BPC_BasicAttack_MaleGreek.AttackReset` (`self.BPC_BasicAttack_MaleGreek`)) ; 공격 중이었다면\n공격을 초기화 시킴
        (`|PlayMontage` (`self.Mesh`) "/Game/Shared_Content/PlayerCharacter/Animation/HammerAnimation/Montages/Roll2.Roll2"
          (:`then`
            (bind (_direction _distancemultiplier) (`Timeline|Movement` :!via `PlayFromStart`)
              (:`Update`
                (bind (_returnvalue_x _returnvalue_y) (`KismetMathLibrary.BreakVector` (* (`self.GetActorForwardVector`) (* _distancemultiplier (`self.MoveDistance`)))))
                (set `MovementComponent.Velocity` (`KismetMathLibrary.MakeVector` _returnvalue_x _returnvalue_y _velocity_z) (`self.CharacterMovement`)))
              (:`Finished`
                (set `self.canDodge` true)))))
        (else
          (set `self.canDodge` true))))))

(event `EnhancedInput|/Game/Shared_Content/Input/IA_MyJump`
  (params (ActionValue :type Boolean) (ElapsedSeconds :type "Float (double-precision)") (TriggeredSeconds :type "Float (double-precision)") (InputAction :type "InputAction Object Reference" :default "/Game/Shared_Content/Input/IA_MyJump.IA_MyJump"))
  ;[1 1 1] Basic Move (기본 동작)
  ;;[1 1 1] Input_Jump
  (:`Triggered`
    (`self.Jump`))
  (:`Completed`
    (`self.StopJumping`)))

(fn `Damage System Event Init`
  (bind _bpc_health (`self.BPC_Health`))
  ;[1 1 1] BPC_DamageSystem에서 발신된 이벤트에, 이벤트함수 연결
  (add `/Game/Shared_Content/DamageSystem/BPC_Health.OnDeath` _bpc_health (`|CreateDelegate` :!event `Death`)) ; OnDeath이벤트에 연결
  (add `/Game/Shared_Content/DamageSystem/BPC_Health.OnBlocked` _bpc_health (`|CreateDelegate` :!event `Blocked`)) ; OnBlocked 이벤트에 연결
  (add `/Game/Shared_Content/DamageSystem/BPC_Health.OnDamaged` _bpc_health (`|CreateDelegate` :!event `Damaged`)) ; OnDamage 이벤트에 연결
)

(fn `GetCurrentHealth`
  (returns (Health :type "Float (double-precision)"))
  (return (`/Game/Shared_Content/DamageSystem/BPC_Health.Health` (`self.BPC_Health`))))

(fn `GetMaxHealth`
  (returns (MaxHealth :type "Float (double-precision)"))
  (return (`/Game/Shared_Content/DamageSystem/BPC_Health.MaxHealth` (`self.BPC_Health`))))

(fn `Heal`
  (params (Amount :type "Float (double-precision)"))
  (returns (NewHealth :type "Float (double-precision)"))
  (bind _newhealth (`/Game/Shared_Content/DamageSystem/BPC_Health.Heal_Execute` (`self.BPC_Health`) Amount))
  (return _newhealth))

(fn `TakeDamage`
  (params (DamageInfo :type "/Game/Shared_Content/DamageSystem/S_DamageRequestInfo Structure"))
  (returns (WasDamaged :type Boolean))
  (bind _wasdamaged (`/Game/Shared_Content/DamageSystem/BPC_Health.TakeDamage_Execute` (`self.BPC_Health`) DamageInfo))
  (return _wasdamaged))

(fn `UpdateCharacterForwrdByCamera`
  (bind (_returnvalue_roll _returnvalue_pitch) (`KismetMathLibrary.BreakRotator` (`self.K2_GetActorRotation` self)))
  ;[1 1 1] 카메라가 바라보는 방향으로, 캐릭터 몸통 회전
  (`self.K2_SetActorRotation` self (`KismetMathLibrary.RInterpTo` (`self.K2_GetActorRotation` self) (`KismetMathLibrary.MakeRotator` _returnvalue_roll _returnvalue_pitch (.yaw (.rotation (`SceneComponent.K2_GetComponentToWorld` (`self.FollowCamera`))))) (`GameplayStatics.GetWorldDeltaSeconds`) 5.0) false))

(fn `Use Stamina`
  (params (requireStaminaAmount :type "Float (double-precision)"))
  (returns (returnIsStaminaEnough :type Boolean))
  (locals (requireStamina :type "Float (double-precision)" :default 10.0) (isStaminaEnough :type Boolean))
  ;[1 1 1] Use Stamina
  (set `local.requireStamina` requireStaminaAmount)
  (if (>= (`self.curStamina`) (`local.requireStamina`))
    (set `self.curStamina` (- (`self.curStamina`) (`local.requireStamina`)))
    (set `local.isStaminaEnough` true)
    (else
      (set `local.isStaminaEnough` false)))
  (return (`local.isStaminaEnough`)))

(fn `UserConstructionScript`
  (bind _bpc_health (`self.BPC_Health`))
  ;[1 1 1] BPC_DamageSystem에서 발신된 이벤트에, 이벤트함수 연결
  (add `/Game/Shared_Content/DamageSystem/BPC_Health.OnDeath` _bpc_health (`|CreateDelegate` :!event `Death`)) ; OnDeath이벤트에 연결
  (add `/Game/Shared_Content/DamageSystem/BPC_Health.OnBlocked` _bpc_health (`|CreateDelegate` :!event `Blocked`)) ; OnBlocked 이벤트에 연결
  (add `/Game/Shared_Content/DamageSystem/BPC_Health.OnDamaged` _bpc_health (`|CreateDelegate` :!event `Damaged`)) ; OnDamageResponse 이벤트에 연결
)