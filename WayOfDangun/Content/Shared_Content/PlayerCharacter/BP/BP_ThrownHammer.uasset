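; Thrown hammer projectile for the player character that strikes enemies, sticks into surfaces and can be recalled.
; Until recall, a short per-tick line trace detects hits: enemies take knockback damage with sound and camera shake as the hammer drops, while other hits freeze it.
; Recall ignores WorldStatic and repeatedly moves toward the player with distance-scaled timing until close, then notifies BPC_HammerThrow_MaleGreek, shows the held hammer and destroys itself.
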(event `ExecuteHammerDetectionTrace`
  (bind _detectionpoint (`self.DetectionPoint`))
  (bind (_returnvalue_x _returnvalue_y _returnvalue_z) (`KismetMathLibrary.BreakVector` (`SceneComponent.K2_GetComponentLocation` _detectionpoint)))
  ;[1 1 1] 망치 탐지 트레이스 처리
  (if (not (`self.isHammerStuck`))
    (bind (_outhit _returnvalue) (`KismetSystemLibrary.LineTraceSingle` (`SceneComponent.K2_GetComponentLocation` _detectionpoint) (`KismetMathLibrary.MakeVector` (+ _returnvalue_x 1.0) _returnvalue_y _returnvalue_z) "TraceTypeQuery5" false (`|MakeArray` (`self.BP_PlayerCharacter`) :!type "Actor Object Reference") "None" true (struct :`R` 1.0 :`A` 1.0) (struct :`G` 1.0 :`A` 1.0) 0.0)) ; 트레이스 생성
    (if _returnvalue
      (bind (_bblockinghit _binitialoverlap _time _distance _location _impactpoint _normal _impactnormal _physmat _hitactor) (`GameplayStatics.BreakHitResult` _outhit))
      (if (`self.ActorHasTag` _hitactor "Enemy")
        (`/Engine/EditorBlueprintResources/StandardMacros.DoOnce` false
          (:`Completed`
            (message `/Game/Shared_Content/DamageSystem/BPI_Damageable.TakeDamage` _hitactor (make `/Game/Shared_Content/DamageSystem/S_DamageRequestInfo` 10.0 "NewEnumerator2" "NewEnumerator2" false true false false false self))
            (`GameplayStatics.PlaySoundAtLocation` "/Game/Shared_Content/PlayerCharacter/SFX/Explosion01.Explosion01" (0.0 0.0 0.0) (struct) 5.0 20.0 0.1 null null null null)
            (`LegacyCameraShake.StartLegacyCameraShake` (`GameplayStatics.GetPlayerCameraManager` 0) "/Game/Shared_Content/PlayerCharacter/CameraShake/BP_CameraShake.BP_CameraShake_C" 10.0 "World")
            (`MovementComponent.StopMovementImmediately` (`self.ProjectileMovement`))
            (set `RotatingMovementComponent.RotationRate` (struct :`Pitch` -120.0 :`Roll` -90.0) (`self.RotatingMovement`))
            (set `ProjectileMovementComponent.ProjectileGravityScale` 10.0 (`self.ProjectileMovement`))
            (`self.ExecuteHammerDetectionTrace`) ; Enemy에 부딪혔으면, 땅/벽에 부딪히기 전까지 다시 시도
          ))
        (else
          (`MovementComponent.StopMovementImmediately` (`self.ProjectileMovement`))
          (set `RotatingMovementComponent.RotationRate` (struct) (`self.RotatingMovement`))
          (set `ProjectileMovementComponent.ProjectileGravityScale` 0.0 (`self.ProjectileMovement`))
          (set `self.isHammerStuck` true))))))

(event `self.ReceiveBeginPlay`
  ;[1 1 1] Event Begin
  ;;[1 1 1] Bp_PlayerCharacter 참조
  (bind _asbp_male_greek (cast `/Game/Shared_Content/PlayerCharacter/BP/BP_MaleGreek` (`GameplayStatics.GetPlayerCharacter` 0)))
  (set `self.BP_PlayerCharacter` _asbp_male_greek)
  (set `self.BPC_HammerThrow_MaleGreek` (`self.GetComponentByClass` (`self.BP_PlayerCharacter`) "/Game/Shared_Content/PlayerCharacter/BP/BPC_HammerThrow_MaleGreek.BPC_HammerThrow_MaleGreek_C")))

(event `self.DetectionPoint.OnComponentHit`
  (params (HitComponent :type "PrimitiveComponent Object Reference") (OtherActor :type "Actor Object Reference") (OtherComp :type "PrimitiveComponent Object Reference") (NormalImpulse :type "Vector Structure") (Hit :type "HitResult Structure (by ref)"))
  ;[1 1 1] 망치 탐지 트레이스 처리
)

(event `self.ReceiveTick`
  (params (DeltaSeconds :type "Float (single-precision)"))
  (bind (_returnvalue_location _returnvalue_rotation) (`KismetMathLibrary.BreakTransform` (`SceneComponent.K2_GetComponentToWorld` (`Character.Mesh` (`self.BP_PlayerCharacter`)))))
  ;[1 1 1] 망치 날라갈때
  ;;[1 1 1] Event Tick
  ;;[1 1 1] 매 프레임마다, 플레이어 위치/회전을 저장
  (set `self.curPlayerLocation` _returnvalue_location)
  (set `self.curPlayerRotator` _returnvalue_rotation)
  (if (not (`self.isRecalling`))
    (`self.ExecuteHammerDetectionTrace`)))

(event `ReturnHammerToPlayer`
  ;[1 1 1] 망치 돌아올 때
  (set `self.isRecalling` true)
  (`/Engine/EditorBlueprintResources/StandardMacros.DoOnce` false
    (:`Completed`
      (`PrimitiveComponent.SetCollisionResponseToChannel` (`self.Hammer`) "ECC_WorldStatic" "ECR_Ignore")
      (`GameplayStatics.PlaySoundAtLocation` "/Game/Shared_Content/PlayerCharacter/SFX/ReceiveFlyingSound.ReceiveFlyingSound" (0.0 0.0 0.0) (struct) 1.5 1.0 0.335 null null null null)
      (`self.Recall_PullHammer`))))

(event `Recall_PullHammer`
  ;[1 1 1] 망치 돌아올 때
  ;;[1 1 1] 가까워질 때까지 망치가 계속 날라옴
  (bind _distance (`self.CalculateDistanceToPlayer`))
  (set `self.curDistanceToPlayer` _distance)
  (bind _output_get (set `self.receivedTime` (/ (`self.curDistanceToPlayer`) 6500.0)))
  (set `/Game/Shared_Content/PlayerCharacter/BP/BPC_HammerThrow_MaleGreek.HammerReceivedTime` _output_get (`self.BPC_HammerThrow_MaleGreek`))
  (`KismetSystemLibrary.MoveComponentTo` (`self.DefaultSceneRoot`) (`self.curPlayerLocation`) (`self.curPlayerRotator`) false true (`self.receivedTime`) true)
  (bind _distance_2 (`self.CalculateDistanceToPlayer`))
  (if (> _distance_2 700.0)
    (set `self.isFirstPulling` false)
    (`self.Recall_PullHammer`)
    (else
      (`/Game/Shared_Content/PlayerCharacter/BP/BPC_HammerThrow_MaleGreek.ReciveHammer` (`self.BPC_HammerThrow_MaleGreek`))
      (`SceneComponent.SetVisibility` (`/Game/Shared_Content/PlayerCharacter/BP/BP_MaleGreek.Hammer` (`self.BP_PlayerCharacter`)) true false)
      (`self.K2_DestroyActor`))))

(fn `CalculateDistanceToPlayer`
  (returns (Distance :type "Float (double-precision)"))
  (return (`KismetMathLibrary.Vector_Distance` (`SceneComponent.K2_GetComponentLocation` (`self.Hammer`)) (`self.curPlayerLocation`))))

(fn `UserConstructionScript`)